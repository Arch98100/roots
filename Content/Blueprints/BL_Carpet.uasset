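; BL_Carpet is a carpet actor that shows popup widgets when something overlaps its collision component.
; While ShowPopup is set, an overlap waits briefly, shows CarpetPopup, clears the flag and swaps the mesh to a carpet runner material.
; Once that flag is clear, an overlap with ShowFinalPopup set shows FinalPopup after a delay and clears that flag.
; The overlapping actor is not filtered.
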(event `self.Collision.OnComponentBeginOverlap`
  (params (OverlappedComponent :type "PrimitiveComponent Object Reference") (OtherActor :type "Actor Object Reference") (OtherComp :type "PrimitiveComponent Object Reference") (OtherBodyIndex :type Integer) (bFromSweep :type Boolean) (SweepResult :type "HitResult Structure (by ref)"))
  (if (`self.ShowPopup`)
    (`KismetSystemLibrary.Delay` 1.0)
    (bind _returnvalue (`|CreateWidget` "/Game/Blueprints/Popups/CarpetPopup.CarpetPopup_C"))
    (`UserWidget.AddToViewport` _returnvalue 0)
    (set `self.ShowPopup` false)
    (`PrimitiveComponent.SetMaterial` (`self.StaticMesh`) 0 "/Game/EF_Edith/Shared/GenericPropsInterior/CarpetRunner/CarpetRunner_a_Mat.CarpetRunner_a_Mat")
    (elif (`self.ShowFinalPopup`)
      (`KismetSystemLibrary.Delay` 2.0)
      (bind _returnvalue_2 (`|CreateWidget` "/Game/Blueprints/Popups/FinalPopup.FinalPopup_C"))
      (`UserWidget.AddToViewport` _returnvalue_2 0)
      (set `self.ShowFinalPopup` false))))

(event `self.Collision.OnComponentEndOverlap`
  (params (OverlappedComponent :type "PrimitiveComponent Object Reference") (OtherActor :type "Actor Object Reference") (OtherComp :type "PrimitiveComponent Object Reference") (OtherBodyIndex :type Integer)))

(fn `UserConstructionScript`)