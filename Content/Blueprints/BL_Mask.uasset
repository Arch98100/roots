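; BL_Mask is an interactable mask pickup that the player collects with the F key.
; Overlapping its collision swaps the mesh to a highlight material and, for the third-person character, enables input and shows a PressF prompt widget; leaving reverses this.
; Pressing F calls FoundPhoto on the player character, destroys the mask and makes the mesh of the MaskWall actor visible.
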(event `self.Collision.OnComponentBeginOverlap`
  (params (OverlappedComponent :type "PrimitiveComponent Object Reference") (OtherActor :type "Actor Object Reference") (OtherComp :type "PrimitiveComponent Object Reference") (OtherBodyIndex :type Integer) (bFromSweep :type Boolean) (SweepResult :type "HitResult Structure (by ref)"))
  (`PrimitiveComponent.SetMaterial` (`self.StaticMesh`) 0 "/Game/Mesh/Bells_Light.Bells_Light")
  (cast `/Game/ThirdPerson/Blueprints/BP_ThirdPersonCharacter` OtherActor)
  (`self.EnableInput` (`GameplayStatics.GetPlayerController` 0))
  (bind _returnvalue (`|CreateWidget` "/Game/Blueprints/PressF.PressF_C"))
  (`UserWidget.AddToViewport` _returnvalue 0))

(event `self.Collision.OnComponentEndOverlap`
  (params (OverlappedComponent :type "PrimitiveComponent Object Reference") (OtherActor :type "Actor Object Reference") (OtherComp :type "PrimitiveComponent Object Reference") (OtherBodyIndex :type Integer))
  (`PrimitiveComponent.SetMaterial` (`self.StaticMesh`) 0 "/Game/EF_Barbra/Materials/BigfootMask_Mat.BigfootMask_Mat")
  (cast `/Game/ThirdPerson/Blueprints/BP_ThirdPersonCharacter` OtherActor)
  (`self.DisableInput` (`GameplayStatics.GetPlayerController` 0))
  (`Widget.RemoveFromParent` (stale `self.Collision.OnComponentBeginOverlap` _returnvalue)))

(event `Key|F`
  (params (Key :type "Key Structure"))
  (:`Pressed`
    (bind _asbp_third_person_character (cast `/Game/ThirdPerson/Blueprints/BP_ThirdPersonCharacter` (`GameplayStatics.GetPlayerPawn` 0)))
    (`/Game/ThirdPerson/Blueprints/BP_ThirdPersonCharacter.foundPhoto` _asbp_third_person_character)
    (`self.K2_DestroyActor`)
    (bind _returnvalue (`GameplayStatics.GetActorOfClass` "/Game/Blueprints/MaskWall.MaskWall_C"))
    (`SceneComponent.SetVisibility` (`/Game/Blueprints/MaskWall.StaticMesh` _returnvalue) true false)))

(fn `UserConstructionScript`)