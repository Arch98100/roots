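; BL_Photo_3 is a collectible photo pickup that the player collects by pressing F.
; Overlapping its collision swaps the mesh to highlight materials and, for BP_ThirdPersonCharacter, enables input and shows a PressF prompt widget.
; Ending the overlap restores the materials, disables input and removes the prompt.
; Pressing F calls FoundPhoto on the character, destroys the pickup and makes the PhotoWall_3 actor's mesh visible.
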(event `self.Collision.OnComponentBeginOverlap`
  (params (OverlappedComponent :type "PrimitiveComponent Object Reference") (OtherActor :type "Actor Object Reference") (OtherComp :type "PrimitiveComponent Object Reference") (OtherBodyIndex :type Integer) (bFromSweep :type Boolean) (SweepResult :type "HitResult Structure (by ref)"))
  (`PrimitiveComponent.SetMaterial` (`self.StaticMesh`) 1 "/Game/Mesh/Picture_4_Light.Picture_4_Light")
  (`PrimitiveComponent.SetMaterial` (`self.StaticMesh`) 0 "/Game/Mesh/Material_Light_Inst.Material_Light_Inst")
  (cast `/Game/ThirdPerson/Blueprints/BP_ThirdPersonCharacter` OtherActor)
  (`self.EnableInput` (`GameplayStatics.GetPlayerController` 0))
  (bind _returnvalue (`|CreateWidget` "/Game/Blueprints/PressF.PressF_C"))
  (`UserWidget.AddToViewport` _returnvalue 0))

(event `self.Collision.OnComponentEndOverlap`
  (params (OverlappedComponent :type "PrimitiveComponent Object Reference") (OtherActor :type "Actor Object Reference") (OtherComp :type "PrimitiveComponent Object Reference") (OtherBodyIndex :type Integer))
  (bind _staticmesh (`self.StaticMesh`))
  (`PrimitiveComponent.SetMaterial` _staticmesh 1 "/Game/Mesh/Picture_Inst.Picture_Inst")
  (`PrimitiveComponent.SetMaterial` _staticmesh 0 "/Game/EF_Barbra/Shared/GenericPropsInterior/PictureFrame/PictureFrameWood_a_Mat.PictureFrameWood_a_Mat")
  (cast `/Game/ThirdPerson/Blueprints/BP_ThirdPersonCharacter` OtherActor)
  (`self.DisableInput` (`GameplayStatics.GetPlayerController` 0))
  (`Widget.RemoveFromParent` (stale `self.Collision.OnComponentBeginOverlap` _returnvalue)))

(event `Key|F`
  (params (Key :type "Key Structure"))
  (:`Pressed`
    (bind _asbp_third_person_character (cast `/Game/ThirdPerson/Blueprints/BP_ThirdPersonCharacter` (`GameplayStatics.GetPlayerPawn` 0)))
    (`/Game/ThirdPerson/Blueprints/BP_ThirdPersonCharacter.foundPhoto` _asbp_third_person_character)
    (`self.K2_DestroyActor`)
    (bind _returnvalue (`GameplayStatics.GetActorOfClass` "/Game/Blueprints/PhotoWall_3.PhotoWall_3_C"))
    (`SceneComponent.SetVisibility` (`/Game/Blueprints/PhotoWall_3.StaticMesh` _returnvalue) true false)))

(fn `UserConstructionScript`)