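; BL_Diary is a collectible pickup that adds one to the third-person character's PhotosFound count and then destroys itself.
; Overlapping its Collision as that character enables input on the actor and shows a Popup widget; leaving disables input and removes the widget.
; Pressing F while input is enabled performs the pickup, without removing the popup in that path.
; The Hint component is hidden at BeginPlay and never shown again here.
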(event `self.ReceiveBeginPlay`
  (`SceneComponent.SetVisibility` (`self.hint`) false false))

(event `self.Collision.OnComponentBeginOverlap`
  (params (OverlappedComponent :type "PrimitiveComponent Object Reference") (OtherActor :type "Actor Object Reference") (OtherComp :type "PrimitiveComponent Object Reference") (OtherBodyIndex :type Integer) (bFromSweep :type Boolean) (SweepResult :type "HitResult Structure (by ref)"))
  (cast `/Game/ThirdPerson/Blueprints/BP_ThirdPersonCharacter` OtherActor)
  (`self.EnableInput` (`GameplayStatics.GetPlayerController` 0))
  (bind _returnvalue (`|CreateWidget` "/Game/Blueprints/Popup.Popup_C"))
  (`UserWidget.AddToViewport` _returnvalue 0))

(event `self.Collision.OnComponentEndOverlap`
  (params (OverlappedComponent :type "PrimitiveComponent Object Reference") (OtherActor :type "Actor Object Reference") (OtherComp :type "PrimitiveComponent Object Reference") (OtherBodyIndex :type Integer))
  (cast `/Game/ThirdPerson/Blueprints/BP_ThirdPersonCharacter` OtherActor)
  (`self.DisableInput` (`GameplayStatics.GetPlayerController` 0))
  (`Widget.RemoveFromParent` (stale `self.Collision.OnComponentBeginOverlap` _returnvalue)))

(event `Key|F`
  (params (Key :type "Key Structure"))
  (:`Pressed`
    (bind _asbp_third_person_character (cast `/Game/ThirdPerson/Blueprints/BP_ThirdPersonCharacter` (`GameplayStatics.GetPlayerPawn` 0)))
    (bind _result (`/Engine/EditorBlueprintResources/StandardMacros.IncrementInt` (`/Game/ThirdPerson/Blueprints/BP_ThirdPersonCharacter.PhotosFound` _asbp_third_person_character))
      (:`  `
        (set `/Game/ThirdPerson/Blueprints/BP_ThirdPersonCharacter.PhotosFound` _result _asbp_third_person_character)
        (`self.K2_DestroyActor`)))))

(fn `UserConstructionScript`)