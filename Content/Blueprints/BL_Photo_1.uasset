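; BL_Photo_1 is a collectible photo pickup that the player collects by pressing F within its collision volume.
; Overlap shows a delayed one-time popup if ShowPopup is set, then enables input and a PressF prompt for the third-person character, both undone on exit.
; Pressing F calls FoundPhoto on the character, destroys the pickup, reveals PhotoWall_1, swaps BL_Carpet to a light material and arms the carpet's popup.
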(event `self.Collision.OnComponentBeginOverlap`
  (params (OverlappedComponent :type "PrimitiveComponent Object Reference") (OtherActor :type "Actor Object Reference") (OtherComp :type "PrimitiveComponent Object Reference") (OtherBodyIndex :type Integer) (bFromSweep :type Boolean) (SweepResult :type "HitResult Structure (by ref)"))
  (if (`self.ShowPopup`)
    (`KismetSystemLibrary.Delay` 1.0)
    (bind _returnvalue (`|CreateWidget` "/Game/Blueprints/Popups/PhotoPopup_1.PhotoPopup_1_C"))
    (`UserWidget.AddToViewport` _returnvalue 10)
    (set `self.ShowPopup` false))
  (cast `/Game/ThirdPerson/Blueprints/BP_ThirdPersonCharacter` OtherActor)
  (`self.EnableInput` (`GameplayStatics.GetPlayerController` 0))
  (bind _returnvalue_2 (`|CreateWidget` "/Game/Blueprints/PressF.PressF_C"))
  (`UserWidget.AddToViewport` _returnvalue_2 0))

(event `self.Collision.OnComponentEndOverlap`
  (params (OverlappedComponent :type "PrimitiveComponent Object Reference") (OtherActor :type "Actor Object Reference") (OtherComp :type "PrimitiveComponent Object Reference") (OtherBodyIndex :type Integer))
  (cast `/Game/ThirdPerson/Blueprints/BP_ThirdPersonCharacter` OtherActor)
  (`self.DisableInput` (`GameplayStatics.GetPlayerController` 0))
  (`Widget.RemoveFromParent` (stale `self.Collision.OnComponentBeginOverlap` _returnvalue_2)))

(event `Key|F`
  (params (Key :type "Key Structure"))
  (:`Pressed`
    (bind _asbp_third_person_character (cast `/Game/ThirdPerson/Blueprints/BP_ThirdPersonCharacter` (`GameplayStatics.GetPlayerPawn` 0)))
    (`/Game/ThirdPerson/Blueprints/BP_ThirdPersonCharacter.foundPhoto` _asbp_third_person_character)
    (`self.K2_DestroyActor`)
    (bind _returnvalue (`GameplayStatics.GetActorOfClass` "/Game/Blueprints/PhotoWall_1.PhotoWall_1_C"))
    (`SceneComponent.SetVisibility` (`/Game/Blueprints/PhotoWall_1.StaticMesh` _returnvalue) true false)
    (bind _returnvalue_2 (`GameplayStatics.GetActorOfClass` "/Game/Blueprints/BL_Carpet.BL_Carpet_C"))
    (`PrimitiveComponent.SetMaterial` (`/Game/Blueprints/BL_Carpet.StaticMesh` _returnvalue_2) 0 "/Game/Mesh/Material_Light_Carpet.Material_Light_Carpet")
    (set `/Game/Blueprints/BL_Carpet.ShowPopup` true _returnvalue_2)))

(fn `UserConstructionScript`)